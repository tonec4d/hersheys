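; BP_Orchestra is a Hersheys orchestra chef Blueprint that drives character animations from number keys.
; Key 1 sets pressed flags on the anim instances of two skeletal meshes and plays a camera shutter sound, then clears the flags on release.
; Key 2 prints a debug string and sets the flag on a third mesh's ABP_2.
; The logic clearing that flag is unconnected, so nothing here resets it.
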(event Input|KeyboardEvents|1
  (params (Key :type Key%20Structure :default "None"))
  (bind _sm_hersheys (Variables|Default|GetSM_Hersheys))
  (bind _sm_hersheys1 (Variables|Default|GetSM_Hersheys1))
  (bind _returnvalue (Components|SkeletalMesh|GetAnimInstance _sm_hersheys1))
  (:Pressed
    (bind _assm_hersheys_skeleton_anim_blueprint (Utilities|Casting|CastToSM_Hersheys_Skeleton_AnimBlueprint (Components|SkeletalMesh|GetAnimInstance _sm_hersheys)))
    (Variables|/Game/Mesh/Hersheys/Orchestra_Chef/SM_Hersheys_Skeleton_AnimBlueprint.SM_Hersheys_Skeleton_AnimBlueprint_C|Setis1pressedanimbp _assm_hersheys_skeleton_anim_blueprint true)
    (bind _asabp_1 (Utilities|Casting|CastToABP_1 _returnvalue))
    (Variables|/Game/Mesh/Hersheys/1/ABP_1.ABP_1_C|SetIs1pressed_player _asabp_1 true)
    (Audio|PlaySound2D "/Engine/VREditor/Sounds/UI/Camera_Shutter.Camera_Shutter" 1.0 1.0 0.0 0 0))
  (:Released
    (bind _assm_hersheys_skeleton_anim_blueprint_2 (Utilities|Casting|CastToSM_Hersheys_Skeleton_AnimBlueprint (Components|SkeletalMesh|GetAnimInstance _sm_hersheys)))
    (Variables|/Game/Mesh/Hersheys/Orchestra_Chef/SM_Hersheys_Skeleton_AnimBlueprint.SM_Hersheys_Skeleton_AnimBlueprint_C|Setis1pressedanimbp _assm_hersheys_skeleton_anim_blueprint_2 false)
    (bind _asabp_1_2 (Utilities|Casting|CastToABP_1 _returnvalue))
    (Variables|/Game/Mesh/Hersheys/1/ABP_1.ABP_1_C|SetIs1pressed_player _asabp_1_2 false)))

(event Input|KeyboardEvents|2
  (params (Key :type Key%20Structure :default "None"))
  (:Pressed
    (Utilities|Casting|CastToABP_2 (Components|SkeletalMesh|GetAnimInstance))
    (Development|PrintString (Utilities|String|ToString(Integer) 0))
    (bind _asabp_2 (Utilities|Casting|CastToABP_2 (Components|SkeletalMesh|GetAnimInstance (Variables|Default|GetSM_Hersheys2))))
    (Variables|/Game/Mesh/Hersheys/2/ABP_2.ABP_2_C|Setis2pressed_player _asabp_2 true)))

(fn ConstructionScript)