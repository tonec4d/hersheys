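; Actor that runs an OSC server to trigger one-shot animations on two Hersheys skeletal meshes from incoming network messages.
; BeginPlay starts the listening server and binds its receive event, which caches each message and address path, then runs four handler functions.
; Each handler matches one item/animation address and plays its animation when the first float equals 1.
; Two debug keys play test animations on the first mesh; leftover print and intensity logic is unconnected.
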(event Custom|OnMsgReceived
  (params (Message :type OSC%20Message%20Structure%20%28by%20ref%29) (IPAddress :type String) (Port :type Integer))
  ;[1 1 1] Binding to Any Message
  (bind _output_get (Variables|Default|SetMessage Message))
  (bind _returnvalue (Class|OSCManager|GetOSCMessageAddress _output_get))
  (bind _returnvalue_2 (Class|OSCManager|GetOSCAddressFullPath _returnvalue))
  (Variables|Default|SetFullPath _returnvalue_2)
  (Utilities|FlowControl|Sequence
    (:then_0
      (Utilities|FlowControl|Sequence
        (:then_1
          (CallFunction|Item2Anim1Func))
        (:then_2
          (CallFunction|Item2Anim2Func))))
    (:then_1
      (CallFunction|Item1Anim1Func))
    (:then_2
      (CallFunction|Item1Anim2Func))))

(event EventBeginPlay
  ;[1 1 1] Binding to Any Message
  (bind _returnvalue (Class|OSCManager|CreateOSCServer (Variables|Default|GetReceive%20IPAddress) (Variables|Default|GetPort) false true "UE_OSC" 0))
  (bind _output_get (Variables|Default|SetTD_OSC_Server _returnvalue))
  (EventDispatchers|AssignOnOscMessageReceived _output_get (delegate Custom|OnMsgReceived)))

(event Collision|EventActorBeginOverlap
  (params (OtherActor :type Actor%20Object%20Reference)))

(event EventTick
  (params (DeltaSeconds :type Float%20%28single-precision%29)))

(event Input|KeyboardEvents|DebugKey1
  (params (Key :type Key%20Structure :default "None") (ActionValue :type Input%20Action%20Value%20Structure))
  (:Pressed
    (Components|Animation|PlayAnimation (Variables|Default|GetSM_Hersheys1) "/Game/Mesh/Hersheys/Hersheys_1_NewSkel/SM_Hersheys_Anim_Armature_Play1Single.SM_Hersheys_Anim_Armature_Play1Single" false)))

(event Input|KeyboardEvents|DebugKey2
  (params (Key :type Key%20Structure :default "None") (ActionValue :type Input%20Action%20Value%20Structure))
  (:Pressed
    (Components|Animation|PlayAnimation (Variables|Default|GetSM_Hersheys1) "/Game/Mesh/Hersheys/Hersheys_1_NewSkel/SM_Hersheys_Anim_Armature_Rest.SM_Hersheys_Anim_Armature_Rest" false)))

(fn ConstructionScript)

(fn Item1Anim1Func
  (if (Class|KismetStringLibrary|MatchesWildcard (Variables|Default|GetFullPath) "/item_1_anim_1" "IgnoreCase")
    (bind _value (Class|OSCManager|GetFloat (Variables|Default|GetMessage)))
    (if (== _value 1.0)
      (Components|Animation|PlayAnimation (Variables|Default|GetSM_Hersheys1) (Variables|Default|GetItem_1_anim_1) false))
    (else
      (Development|PrintString "False1"))))

(fn Item1Anim2Func
  (if (Class|KismetStringLibrary|MatchesWildcard (Variables|Default|GetFullPath) "/item_1_anim_2" "IgnoreCase")
    (bind _value (Class|OSCManager|GetFloat (Variables|Default|GetMessage)))
    (if (== _value 1.0)
      (Components|Animation|PlayAnimation (Variables|Default|GetSM_Hersheys1) (Variables|Default|GetItem_1_anim_2) false))
    (else
      (Development|PrintString "False1"))))

(fn Item2Anim1Func
  (if (Class|KismetStringLibrary|MatchesWildcard (Variables|Default|GetFullPath) "/item_2_anim_1" "IgnoreCase")
    (bind _value (Class|OSCManager|GetFloat (Variables|Default|GetMessage)))
    (if (== _value 1.0)
      (Components|Animation|PlayAnimation (Variables|Default|GetSM_Hersheys2) (Variables|Default|GetIteam_2_anim_1) false))
    (else
      (Development|PrintString "False1"))))

(fn Item2Anim2Func
  (if (Class|KismetStringLibrary|MatchesWildcard (Variables|Default|GetFullPath) "/item_2_anim_2" "IgnoreCase")
    (bind _value (Class|OSCManager|GetFloat (Variables|Default|GetMessage)))
    (if (== _value 1.0)
      (Components|Animation|PlayAnimation (Variables|Default|GetSM_Hersheys2) (Variables|Default|GetItem_2_anim_2) false))
    (else
      (Development|PrintString "False1"))))